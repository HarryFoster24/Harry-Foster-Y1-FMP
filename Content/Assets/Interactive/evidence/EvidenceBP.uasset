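; EvidenceBP is a collectible evidence pickup that advances the player's objective.
; When a FirstPersonCharacter overlaps its Box, it increments that character's EvidenceAmount and destroys itself.
; Each tick it checks the player's EvidenceAmount and, once it reaches at least four, sets ObjectiveTask to escape through the balcony.
; Because that check lives on each pickup, it only runs while an evidence actor still exists.
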(event `self.ReceiveBeginPlay`)

(event `self.ReceiveTick`
  (params (DeltaSeconds :type "Float (single-precision)"))
  (bind _asfirst_person_character (cast `/Game/FirstPersonBP/Blueprints/FirstPersonCharacter` (`GameplayStatics.GetPlayerCharacter` 0)))
  (if (>= (`/Game/FirstPersonBP/Blueprints/FirstPersonCharacter.evidenceAmount` _asfirst_person_character) 4)
    (set `/Game/FirstPersonBP/Blueprints/FirstPersonCharacter.objectiveTask` "ESCAPE THROUGH BALCONY" _asfirst_person_character)))

(event `self.Box.OnComponentBeginOverlap`
  (params (OverlappedComponent :type "PrimitiveComponent Object Reference") (OtherActor :type "Actor Object Reference") (OtherComp :type "PrimitiveComponent Object Reference") (OtherBodyIndex :type Integer) (bFromSweep :type Boolean) (SweepResult :type "HitResult Structure (by ref)"))
  (bind _asfirst_person_character (cast `/Game/FirstPersonBP/Blueprints/FirstPersonCharacter` OtherActor))
  (set `/Game/FirstPersonBP/Blueprints/FirstPersonCharacter.evidenceAmount` (+ 1 (`/Game/FirstPersonBP/Blueprints/FirstPersonCharacter.evidenceAmount` _asfirst_person_character)) _asfirst_person_character)
  (`self.K2_DestroyActor`))

(fn `UserConstructionScript`)