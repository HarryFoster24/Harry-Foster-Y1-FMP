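; Interactive hinged door Blueprint (drawBP) that the player opens and closes with the F key.
; Overlapping the front hitbox as a FirstPersonCharacter enables input on the actor and shows an InteractWidget prompt; leaving disables input and removes the widget.
; Each F press flip-flops a timeline between play and reverse, driving the yaw of DoorPivot's relative rotation.
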(event `self.fronthitbox.OnComponentBeginOverlap`
  (params (OverlappedComponent :type "PrimitiveComponent Object Reference") (OtherActor :type "Actor Object Reference") (OtherComp :type "PrimitiveComponent Object Reference") (OtherBodyIndex :type Integer) (bFromSweep :type Boolean) (SweepResult :type "HitResult Structure (by ref)"))
  ;[1 1 1] Enables Input when near Door
  (cast `/Game/FirstPersonBP/Blueprints/FirstPersonCharacter` OtherActor)
  (`self.EnableInput` (`GameplayStatics.GetPlayerController` 0))
  (bind _returnvalue (`|CreateWidget` "/Game/Widgets/interactWidget.interactWidget_C"))
  (`UserWidget.AddToViewport` _returnvalue 0))

(event `self.fronthitbox.OnComponentEndOverlap`
  (params (OverlappedComponent :type "PrimitiveComponent Object Reference") (OtherActor :type "Actor Object Reference") (OtherComp :type "PrimitiveComponent Object Reference") (OtherBodyIndex :type Integer))
  ;[1 1 1] Enables Input when near Door
  (cast `/Game/FirstPersonBP/Blueprints/FirstPersonCharacter` OtherActor)
  (`self.DisableInput` (`GameplayStatics.GetPlayerController` 0))
  (bind _foundwidgets (`WidgetBlueprintLibrary.GetAllWidgetsOfClass` "/Game/Widgets/interactWidget.interactWidget_C"))
  (`Widget.RemoveFromParent` _foundwidgets))

(event `Key|F`
  (params (Key :type "Key Structure"))
  ;[1 1 1] Door open/close for player & AI
  (:`Pressed`
    (`/Engine/EditorBlueprintResources/StandardMacros.FlipFlop`
      (:`A`
        (bind (_direction _rotatedoor) (`Timeline|FrontDoorTimeLine` :!label _label)
          (:`Update`
            (`SceneComponent.K2_SetRelativeRotation` (`self.doorPivot`) (`KismetMathLibrary.MakeRotator` 0.0 0.0 _rotatedoor) false false))))
      (:`B`
        (goto _label :!via `Reverse`)))))

(fn `UserConstructionScript`)